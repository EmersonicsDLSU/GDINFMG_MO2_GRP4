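; DatabaseHelper is a Blueprint helper that wraps MySQL connection and query calls and reports their results through callbacks.
; GetData stores the query and starts GetData_INTERNAL by name as an async function, which queries over the stored connection and reports success, with Found always false and rows unused.
; CreateDatabase_INTERNAL opens and stores the connection, but ConnectToDatabase passes an empty function name, so it does not reference that event.
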(event `GetData`
  (params (Query :type String))
  (set `self.Query` Query)
  (`FuncCaller.StartAsyncFuncByFuncName` "GetData_INTERNAL" self))

(event `GetData_INTERNAL`
  (bind _result_rows (`/MySQLConnectorUE4Plugin/Blueprints/Macros/SQLDatabaseMacros.MySQL_Execute_Query_With_Result` (`self.Query`) (`self.DatabaseConnection`))
    (:`Success`
      (`self.OnGetData` true))
    (:`Error`
      (`self.OnGetData` false))))

(event `ConnectToDatabase`
  (`FuncCaller.StartAsyncFuncByFuncName` "" self))

(event `CreateDatabase_INTERNAL`
  (bind _connection (`/MySQLConnectorUE4Plugin/Blueprints/Macros/SQLDatabaseMacros.MySQL_Connect` "")
    (:`Success`
      (bind _output_get (set `self.DatabaseConnection` _connection))
      (`self.OnConnectionResult` true _output_get))
    (:`Error`
      (`self.OnConnectionResult` false))))